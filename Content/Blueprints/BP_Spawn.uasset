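; BP_Spawn is the breakable cube grid of a ball-and-brick game, ending the game when every cube is destroyed.
; The construction script builds static mesh components in an X/Y grid spaced by Padding; BeginPlay randomizes their materials and creates the BP_Widget counter.
; Materials double as hit points: each Ball hit increments the counter and steps the material down, destroying cubes at the lowest tier.
; Clearing the last cube pauses and shows the game-over screen.
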(event EventBeginPlay
  (bind _arraycomp (Variables|Components|GetArrayComp))
  (for _index (range 0 (- (Utilities|Array|Length _arraycomp) 1))
    (Rendering|Material|SetMaterial (Utilities|Array|Get(acopy) _arraycomp _index) 0 (Utilities|Array|Get(acopy) (Variables|Components|GetArrayMat) (Math|Random|RandomIntegerinRange 0 2))))
  (bind _returnvalue (UserInterface|CreateWidget "/Game/Blueprints/BP_Widget.BP_Widget_C"))
  (UserInterface|Viewport|AddtoViewport _returnvalue 0)
  (Variables|/Game/Blueprints/BP_Widget.BP_Widget_C|SetBP_Spawn_Var _returnvalue self)
  (bind _output_get (Variables|Components|SetBP_Widget _returnvalue))
  (Default|UpdateCounter _output_get))

(event Collision|EventActorBeginOverlap
  (params (OtherActor :type Actor%20Object%20Reference)))

(event EventTick
  (params (DeltaSeconds :type Float%20%28single-precision%29)))

(event Collision|EventHit
  (params (MyComp :type Primitive%20Component%20Object%20Reference) (Other :type Actor%20Object%20Reference) (OtherComp :type Primitive%20Component%20Object%20Reference) (bSelfMoved :type Boolean) (HitLocation :type Vector :default "0, 0, 0") (HitNormal :type Vector :default "0, 0, 0") (NormalImpulse :type Vector :default "0, 0, 0") (Hit :type Hit%20Result%20Structure%20%28by%20ref%29))
  (bind _arraymat (Variables|Components|GetArrayMat))
  (bind _cubescount (Variables|Components|GetCubesCount))
  (Utilities|Casting|CastToBall Other)
  (Math|Integer|IncrementInt (Variables|Components|GetDest_Count)
    (:%20%20
      (Default|UpdateCounter (Variables|Components|GetBP_Widget))
      (if (== (Rendering|Material|GetMaterial MyComp 0) (Utilities|Array|Get(acopy) _arraymat 2))
        (Rendering|Material|SetMaterial MyComp 0 (Utilities|Array|Get(acopy) (Variables|Components|GetArrayMat) 1))
        (elif (== (Rendering|Material|GetMaterial MyComp 0) (Utilities|Array|Get(acopy) _arraymat 1))
          (Rendering|Material|SetMaterial MyComp 0 (Utilities|Array|Get(acopy) (Variables|Components|GetArrayMat)))
          (elif (== (Rendering|Material|GetMaterial MyComp 0) (Utilities|Array|Get(acopy) _arraymat))
            (Components|DestroyComponent MyComp)
            (Math|Integer|DecrementInt _cubescount
              (:%20%20
                (if (== _cubescount 0)
                  (Game|SetGamePaused true)
                  (Default|GameOverScreen (Variables|Components|GetBP_Widget)))))))))))

(fn ConstructionScript
  (Variables|Components|SetCubesCount 0)
  (Utilities|Array|Resize (Variables|Components|GetArrayComp) (* (+ (Variables|Components|GetX) 1) (+ (Variables|Components|GetY) 1)))
  (for _index (range 0 (Variables|Components|GetY))
    (for _index_2 (range 0 (Variables|Components|GetX))
      (bind _returnvalue (AddComponent|AddStaticMeshComponent false (Math|Transform|MakeTransform (Math|Vector|MakeVector (Math|Conversions|ToFloat(Integer) (* _index_2 (Variables|Components|GetPadding))) (Math|Conversions|ToFloat(Integer) (* _index (Variables|Components|GetPadding))) 0.0))))
      (Utilities|Array|SetArrayElem (Variables|Components|GetArrayComp) (Variables|Components|GetCubesCount) _returnvalue)
      (Math|Integer|IncrementInt (Variables|Components|GetCubesCount)))))