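; Ball actor that bounces around the level and, on overlapping a KillZVolume, destroys itself and calls Respawn on the first BP_Pawn.
; Tick sweeps it along its Speed vector, mirroring that vector off the hit normal on blocking hits and adding random X variation.
; Pillar destruction, Game_Over pause and quit logic are present but disconnected, so they never run.
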(event EventBeginPlay)

(event Collision|EventActorBeginOverlap
  (params (OtherActor :type Actor%20Object%20Reference))
  (Utilities|Casting|CastToKillZVolume OtherActor)
  (Actor|DestroyActor)
  (bind _outactors (Actor|GetAllActorsOfClass "/Game/Blueprints/BP_Pawn.BP_Pawn_C"))
  (Default|Respawn (Utilities|Array|Get(acopy) _outactors)))

(event EventTick
  (params (DeltaSeconds :type Float%20%28single-precision%29))
  (bind _sweephitresult (Transformation|AddActorWorldOffset (* DeltaSeconds (Variables|Default|GetSpeed)) true))
  (if (.bBlockingHit (Collision|BreakHitResult _sweephitresult))
    (Variables|Default|SetSpeed (Math|Vector|MakeVector (+ (Math|Random|RandomFloatinRange -2.0 2.0) (.X (Math|Vector|BreakVector (Math|Vector|MirrorVectorbyNormal (Variables|Default|GetSpeed) (Math|Vector|MakeVector (.X (Math|Vector|BreakVector (.Normal (Collision|BreakHitResult _sweephitresult)))) (.Y (Math|Vector|BreakVector (.Normal (Collision|BreakHitResult _sweephitresult)))) 0.0))))) (.Y (Math|Vector|BreakVector (Math|Vector|MirrorVectorbyNormal (Variables|Default|GetSpeed) (Math|Vector|MakeVector (.X (Math|Vector|BreakVector (.Normal (Collision|BreakHitResult _sweephitresult)))) (.Y (Math|Vector|BreakVector (.Normal (Collision|BreakHitResult _sweephitresult)))) 0.0)))) (.Z (Math|Vector|BreakVector (Math|Vector|MirrorVectorbyNormal (Variables|Default|GetSpeed) (Math|Vector|MakeVector (.X (Math|Vector|BreakVector (.Normal (Collision|BreakHitResult _sweephitresult)))) (.Y (Math|Vector|BreakVector (.Normal (Collision|BreakHitResult _sweephitresult)))) 0.0))))))))

(fn ConstructionScript)