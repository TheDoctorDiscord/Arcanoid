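; Traffic light actor that blinks its Red, Yellow and Green components in turn, in an endless cycle.
; The construction script collects the three components into an array.
; From BeginPlay, a Delay-driven loop toggles the current component's visibility every Time seconds.
; A countdown reset from Count sets how many toggles each light gets before the index advances and wraps back to Red.
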(event EventBeginPlay
  (Variables|Default|SetCountNonPub (Variables|Default|GetCount))
  (Utilities|FlowControl|Delay (Variables|Default|GetTime) :!label _label)
  (Rendering|ToggleVisibility (Utilities|Array|Get(acopy) (Variables|Default|GetArray1) (Variables|Default|GetId)) false)
  (if (< (Variables|Default|GetCountNonPub) 0)
    (Variables|Default|SetCountNonPub (Variables|Default|GetCount))
    (Math|Integer|IncrementInt (Variables|Default|GetId)
      (:%20%20
        (if (< (Variables|Default|GetId) 3)
          (goto _label)
          (else
            (Variables|Default|SetId 0)
            (goto _label)))))
    (else
      (Math|Integer|DecrementInt (Variables|Default|GetCountNonPub)
        (:%20%20
          (goto _label))))))

(event Collision|EventActorBeginOverlap
  (params (OtherActor :type Actor%20Object%20Reference)))

(event EventTick
  (params (DeltaSeconds :type Float%20%28single-precision%29)))

(fn ConstructionScript
  (bind _array1 (Variables|Default|GetArray1))
  (Utilities|Array|Add _array1 (Variables|Default|GetRed))
  (Utilities|Array|Add _array1 (Variables|Default|GetYellow))
  (Utilities|Array|Add _array1 (Variables|Default|GetGreen)))